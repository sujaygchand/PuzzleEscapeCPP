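; BP_Door is a door actor that swings open and closed in response to requests from its OpenDoor member.
; It caches its starting rotation at BeginPlay, and open and close requests play or reverse the RotateDoor timeline.
; Each timeline update combines the OpenAngle yaw with that initial rotation, while a Sound Timing event track plays the Doorlock sound at the door's location.
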(event `self.ReceiveBeginPlay`
  (set `self.Initial Rotation` (`self.K2_GetActorRotation`)))

(event `self.OpenDoor.OnOpenRequest`
  ;[1 1 1] Opens and closes door
  (bind (_direction _openangle) (`Timeline|RotateDoor` :!label _label)
    (:`Update`
      (`self.K2_SetActorRotation` (`KismetMathLibrary.ComposeRotators` (`KismetMathLibrary.MakeRotator` 0.0 0.0 _openangle) (`self.Initial Rotation`))))
    (:`SoundTiming`
      (`GameplayStatics.PlaySoundAtLocation` "/Game/Sounds/door-lock.door-lock" (`self.K2_GetActorLocation`)))))

(event `self.OpenDoor.OnCloseRequest`
  ;[1 1 1] Opens and closes door
  (goto _label :!via `Reverse`))

(fn `UserConstructionScript`)